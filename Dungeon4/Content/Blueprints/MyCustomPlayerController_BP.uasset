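; A player controller Blueprint that relays health and room progress to the MainHUD.
; UpdateHealthBar casts the HUD to MainHUD and passes Health divided by MaxHealth, printing a warning if the cast fails.
; UpdateRoomNumber uses the same cast to pass CurrentRoomNumber, stopping silently on failure.
; BeginPlay, Tick and the construction script do nothing, so updates run only when these events are called.
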(event `self.UpdateHealthBar`
  (bind _asmain_hud (cast `/Game/UI/HUD/MainHUD` (`self.HUD`))
    (:`then`
      (`/Game/UI/HUD/MainHUD.UpdateHealthBar` _asmain_hud (/ (`self.Health`) (`self.MaxHealth`))))
    (:`CastFailed`
      (`KismetSystemLibrary.PrintString` "HUD not Found"))))

(event `self.UpdateRoomNumber`
  (bind _asmain_hud (cast `/Game/UI/HUD/MainHUD` (`self.HUD`)))
  (`/Game/UI/HUD/MainHUD.UpdateCurrentRoom` _asmain_hud (`self.CurrentRoomNumber`)))

(fn `UserConstructionScript`)