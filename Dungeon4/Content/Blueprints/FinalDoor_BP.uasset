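; FinalDoor_BP is a child Blueprint for the final door, which registers itself with the game mode.
; On BeginPlay it runs the parent logic, casts the game mode to PlayerTesting and stores itself as LastDoor.
; Its UpdateEnemiesRemaining event is empty, and the overlap and tick events are disabled stubs, so the registration is its only added logic.
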(event `self.ReceiveBeginPlay`
  (`parent.ReceiveBeginPlay`)
  (bind _asplayer_testing (cast `/Game/GameModes/PlayerTesting` (`GameplayStatics.GetGameMode`)))
  (set `/Game/GameModes/PlayerTesting.LastDoor` self _asplayer_testing))

(event `UpdateEnemiesRemaining`)

(fn `UserConstructionScript`
  (`parent.UserConstructionScript`))