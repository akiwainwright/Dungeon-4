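; Greater spider enemy that chases and attacks the player, with a health bar widget showing its health ratio.
; Events drive pursuit through the enemy controller and play Attack or Defeat sections of one montage after stopping movement.
; The arm collider starts disabled; its overlap triggers the player's effect, passes Attack to the player controller's health update and plays a hit sound.
; A separate event spawns a coin-burst particle system as damage feedback.
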(event `self.ReceiveBeginPlay`
  (bind _asenemy_health_bar (cast `/Game/UI/HUD/EnemyHealthBar` (`WidgetComponent.GetWidget` (`self.HealthWidget`))))
  (`ProgressBar.SetPercent` (`/Game/UI/HUD/EnemyHealthBar.EnemyHealth` _asenemy_health_bar) (/ (`self.Health`) (`self.MaxHealth`)))
  (`PrimitiveComponent.SetCollisionEnabled` (`self.ArmCollider`) "NoCollision"))

(event `self.UpdateHealthBar`
  (bind _asenemy_health_bar (cast `/Game/UI/HUD/EnemyHealthBar` (`WidgetComponent.GetWidget` (`self.HealthWidget`))))
  (`ProgressBar.SetPercent` (`/Game/UI/HUD/EnemyHealthBar.EnemyHealth` _asenemy_health_bar) (/ (`self.Health`) (`self.MaxHealth`))))

(event `self.PursuePlayer`
  (params (PursueTarget :type "Actor Object Reference"))
  (`AIController.MoveToActor` (`self.EnemyController`) PursueTarget 20.0 true true true null true))

(event `self.StopPursuing`
  (`Controller.StopMovement` (`self.EnemyController`)))

(event `self.AttackPlayer`
  (bind _returnvalue (`SkeletalMeshComponent.GetAnimInstance` (`self.Mesh`)))
  (`Controller.StopMovement` (`self.EnemyController`))
  (`AnimInstance.Montage_Play` _returnvalue "/Game/Enemies/GreatSpider/GreatSpiderFightMontage.GreatSpiderFightMontage" 1.0 "MontageLength" 0.0 true)
  (`AnimInstance.Montage_JumpToSection` _returnvalue "Attack" "/Game/Enemies/GreatSpider/GreatSpiderFightMontage.GreatSpiderFightMontage"))

(event `self.ArmCollider.OnComponentBeginOverlap`
  (params (OverlappedComponent :type "PrimitiveComponent Object Reference") (OtherActor :type "Actor Object Reference") (OtherComp :type "PrimitiveComponent Object Reference") (OtherBodyIndex :type Integer) (bFromSweep :type Boolean) (SweepResult :type "HitResult Structure (by ref)"))
  (bind _asplayer_character_bp (cast `/Game/Blueprints/PlayerCharacter_BP` OtherActor))
  (`PlayerCharacter.StartPlayingEffect` _asplayer_character_bp (`SceneComponent.K2_GetComponentLocation` OverlappedComponent))
  (bind _asmy_custom_player_controller_bp (cast `/Game/Blueprints/MyCustomPlayerController_BP` (`self.GetController` _asplayer_character_bp)))
  (`CustomPlayerController.UpdateHealth` _asmy_custom_player_controller_bp (`self.Attack`))
  (`GameplayStatics.PlaySound2D` "/Game/Audio/SoundCues/Hit2_Cue.Hit2_Cue" 1.0 1.0 0.0 null null))

(event `self.DeathSequence`
  (bind _returnvalue (`SkeletalMeshComponent.GetAnimInstance` (`self.Mesh`)))
  (`Controller.StopMovement` (`self.EnemyController`))
  (`AnimInstance.Montage_Play` _returnvalue "/Game/Enemies/GreatSpider/GreatSpiderFightMontage.GreatSpiderFightMontage" 1.0 "MontageLength" 0.0 true)
  (`AnimInstance.Montage_JumpToSection` _returnvalue "Defeat" "/Game/Enemies/GreatSpider/GreatSpiderFightMontage.GreatSpiderFightMontage"))

(event `self.PlayDamageEffect`
  (params (Location :type "Vector Structure"))
  (`NiagaraFunctionLibrary.SpawnSystemAtLocation` "/Game/sA_PickupSet_1/Fx/NiagaraSystems/NS_CoinBurst_2.NS_CoinBurst_2" Location))

(fn `UserConstructionScript`)