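; Troll enemy character that carries a weapon and can chase a target on request.
; On BeginPlay it spawns a TrollWeapon_BP and snaps it to the right-hand weapon socket on its mesh.
; PursuePlayer and StopPursuing events drive its EnemyController to move to the given actor or halt, with no calls to them in this graph.
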(event `self.ReceiveBeginPlay`
  (bind _returnvalue (`|SpawnActorFromClass` "/Game/Enemies/Troll/TrollWeapon_BP.TrollWeapon_BP_C" (`SceneComponent.GetSocketTransform` (`self.Mesh`) "b_MF_Weapon_R_Socket" "RTS_World") "Undefined" "OverrideRootScale" null null))
  (`self.K2_AttachToComponent` _returnvalue (`self.Mesh`) "b_MF_Weapon_R_Socket" "SnapToTarget" "SnapToTarget" "SnapToTarget" true))

(event `self.PursuePlayer`
  (params (PursueTarget :type "Actor Object Reference"))
  (`AIController.MoveToActor` (`self.EnemyController`) PursueTarget 40.0 true true true null true))

(event `self.StopPursuing`
  (`Controller.StopMovement` (`self.EnemyController`)))

(fn `UserConstructionScript`)